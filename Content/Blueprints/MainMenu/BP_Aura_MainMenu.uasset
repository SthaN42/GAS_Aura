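; BP_Aura_MainMenu is a main menu scene actor that sets up the menu and animates its backdrop.
; On BeginPlay it records the fireball's start location, plays the menu music, adds WBP_MainMenu to the viewport and switches to UI-only input with a visible cursor.
; Each Tick bobs the fireball vertically on a sine of accumulated time and rotates the magic circle decal at a set rate.
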(event EventBeginPlay
  (Variables|Default|SetInitialFireballLoc (Transformation|GetWorldLocation (Variables|Default|GetFireball)))
  (Audio|SpawnSound2D "/Game/Assets/Sounds/Music/Music_MainMenu.Music_MainMenu" 0.5 1.0 0.0 0)
  (bind _returnvalue (UserInterface|CreateWidget "/Game/Blueprints/UI/MainMenu/WBP_MainMenu.WBP_MainMenu_C"))
  (Utilities|IsValid _returnvalue
    (:Is%20Valid
      (UserInterface|Viewport|AddtoViewport _returnvalue 0)
      (Input|SetInputModeUIOnly (Game|GetPlayerController 0) 0 "DoNotLock" false)
      (Variables|/Script/Engine.PlayerController|SetbShowMouseCursor (Game|GetPlayerController 0) true))))

(event EventTick
  (params (DeltaSeconds :type Float%20%28single-precision%29))
  (bind _output_get (Variables|Default|SetTime (+ DeltaSeconds (Variables|Default|GetTime))))
  (Transformation|SetWorldLocation (Variables|Default|GetFireball) (+ (Variables|Default|GetInitialFireballLoc) (Math|Vector|MakeVector 0.0 0.0 (* (Math|Trig|Sin(Radians) _output_get) (Variables|Default|GetMagnitude)))) false false)
  (Transformation|AddLocalRotation (Variables|Default|GetDecal) (Math|Rotator|MakeRotator (* (Utilities|Time|GetWorldDeltaSeconds) (Variables|Default|GetMagicCircleRotationRate)) 0.0 0.0) false false))

(fn ConstructionScript)