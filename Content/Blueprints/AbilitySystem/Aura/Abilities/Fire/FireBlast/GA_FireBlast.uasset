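; Gameplay ability for Fire Blast, a spell described as launching fire balls in all directions that return and explode for radial fire damage with a burn chance.
; On activation it commits, calls SpawnFireBalls, which is defined outside these graphs, and ends immediately.
; Current and next-level descriptions are rich-text strings filled from level-based mana cost, cooldown and damage, plus the fire ball count.
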(event Ability|EventActivateAbility
  (Ability|CommitAbility)
  (Class|AuraFireBlast|SpawnFireBalls)
  (Ability|EndAbility))

(event Ability|EventOnEndAbility
  (params (bWasCancelled :type Boolean)))

(fn GetDescription
  (params (Level :type Integer))
  (return (Utilities|String|ToString(Text) (Utilities|Text|FormatText "<Title>FIRE BLAST</> 
<Small>Level   </><Level>{Level}</> 
<Small>Mana Cost   </><ManaCost>{ManaCost}</> 
<Small>Cooldown   </><Cooldown>{Cooldown}s</> 
 
<Default>Launches </><Number>{NumBalls}</><Default> fire balls in all directions, each coming back and exploding upon return, causing </><Damage>{Damage}</><Default> radial fire damage with a chance to burn.</>" Level (Class|AuraGameplayAbility|GetManaCost (Math|Conversions|ToFloat(Integer) Level)) (Class|AuraGameplayAbility|GetCooldown (Math|Conversions|ToFloat(Integer) Level)) (Variables|Default|GetNumFireBalls) (Math|Float|Truncate (Class|AuraDamageGameplayAbility|GetDamage (Math|Conversions|ToFloat(Integer) Level)))))))

(fn GetNextLevelDescription
  (params (Level :type Integer))
  (return (Utilities|String|ToString(Text) (Utilities|Text|FormatText "<Title>NEXT LEVEL</> 
<Small>Level   </><Level>{Level}</> 
<Small>Mana Cost   </><ManaCost>{ManaCost}</> 
<Small>Cooldown   </><Cooldown>{Cooldown}s</> 
 
<Default>Launches </><Number>{NumBalls}</><Default> fire balls in all directions, each coming back and exploding upon return, causing </><Damage>{Damage}</><Default> radial fire damage with a chance to burn.</>" Level (Class|AuraGameplayAbility|GetManaCost (Math|Conversions|ToFloat(Integer) Level)) (Class|AuraGameplayAbility|GetCooldown (Math|Conversions|ToFloat(Integer) Level)) (Variables|Default|GetNumFireBalls) (Math|Float|Truncate (Class|AuraDamageGameplayAbility|GetDamage (Math|Conversions|ToFloat(Integer) Level)))))))