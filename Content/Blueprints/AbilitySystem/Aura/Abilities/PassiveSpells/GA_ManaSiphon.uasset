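; GA_ManaSiphon is the Mana Siphon passive gameplay ability for Aura, currently a stub with no siphon effect in its graphs.
; Activation and end events only print the ability's display name with an Activated or Ended suffix.
; GetDescription returns a rich-text title with the spell level, while GetNextLevelDescription returns an empty string.
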(event Ability|EventActivateAbility
  (Development|PrintString (Utilities|String|Append (Utilities|GetDisplayName self) " Activated") true true "(R=0.000000,G=1.000000,B=0.000000,A=1.000000)"))

(event Ability|EventOnEndAbility
  (params (bWasCancelled :type Boolean))
  (Development|PrintString (Utilities|String|Append (Utilities|GetDisplayName self) " Ended") true true "(R=1.000000,G=0.000000,B=0.000000,A=1.000000)"))

(fn GetDescription
  (params (Level :type Integer))
  (return (Utilities|String|ToString(Text) (Utilities|Text|FormatText "<Title>MANA SIPHON</> 
<Small>Level   </><Level>{Level}</> 
 
<Default></>" Level))))

(fn GetNextLevelDescription
  (params (Level :type Integer))
  (return ""))