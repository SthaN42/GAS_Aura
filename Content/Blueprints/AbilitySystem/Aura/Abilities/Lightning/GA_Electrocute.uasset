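; Electrocute lightning ability: a channeled beam at the target under the mouse that chains to nearby enemies at higher levels.
; A montage event locks movement, adds ShockLoop cues on targets and starts a looping timer that commits cost and deals damage, ending when cost fails.
; Input release ends it and starts cooldown, with a server-side delay enforcing minimum cast time.
; On ending, the server applies final damage with debuff chance.
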(event Custom|DamageAndCost
  ;[0 1 0.08594] Periodically check if we can commit the cost. If we can, apply damage. Else, end the ability
  (bind _returnvalue (Ability|CommitAbilityCost false))
  (if _returnvalue
    (CallFunction|ApplyDamage)
    (else
      (CallFunction|ClearandEndAbility))))

(event Ability|EventActivateAbility
  (CallFunction|EnforceImplementsCombatInterface)
  ;[1 0 0.7969] Store target data variables
  (bind _datahandle (|TargetDataUnderMouse)
    (:ValidData
      (if (.bBlockingHit (Collision|BreakHitResult (Ability|TargetData|GetHitResultfromTargetData _datahandle)))
        (Class|AuraBeamSpell|StoreMouseDataInfo (Ability|TargetData|GetHitResultfromTargetData _datahandle))
        (Class|AuraBeamSpell|StoreOwnerVariables)
        (Utilities|FlowControl|Sequence
          (:then_0
            (CallFunction|PreparetoStartAbility)
            (GameplayCue|ExecuteGameplayCue :GameplayCueTag "(TagName=\"GameplayCue.SockBurst\")")
            (|PlayMontageandWaitProxy "None" (Variables|Default|GetMontage_Electrocute) 1.0 "None" true 1.0 0.0 false
              (:then
                (Ability|Tasks|WaitGameplayEvent "(TagName=\"Event.Montage.Electrocute\")" 0 true
                  (:EventReceived
                    (CallFunction|InShockLoop)
                    (CallFunction|SpawnElectricBeam)
                    ;[0 1 0.08594] Periodically check if we can commit the cost. If we can, apply damage. Else, end the ability
                    (bind _returnvalue (Utilities|Time|SetTimerbyEvent (delegate Custom|DamageAndCost) (Variables|Default|GetDamageDeltaTime) true))
                    (Variables|Default|SetDamageAndCostTimer _returnvalue))))))
          (:then_1
            ;[0 0.7891 1] Enforce a minimum spell time, to prevent weird thins from happening when pressing the input not long enough
            (bind _timeheld (Ability|Tasks|WaitInputRelease false)
              (:OnRelease
                (bind _output_get (Variables|Default|SetTimeHeld _timeheld))
                (if (< _output_get (Variables|Default|GetMinSpellTime))
                  (Ability|HasAuthority
                    (:True
                      (Utilities|FlowControl|Delay (- (Variables|Default|GetMinSpellTime) (Variables|Default|GetTimeHeld)))
                      (CallFunction|ClearandEndAbility))
                    (:False
                      (CallFunction|PreparetoEndAbility)))
                  (else
                    (CallFunction|ClearandEndAbility)))))))
        (else
          ;[0 1 0.5547] Cancel the abiltiy if we click in the void
          (Ability|CancelAbility))))))

(event EventPrimaryTargetDied
  (params (DeadActor :type Actor%20Object%20Reference))
  ;[1 0.3886 0] Primary Target Died. We are done
  (CallFunction|ClearandEndAbility))

(event EventAdditionalTargetDied
  (params (DeadActor :type Actor%20Object%20Reference))
  ;[1 0.3886 0] Additional Target Died. Remove it from Additional Targets and Shock Loop Cue
  (CallFunction|RemoveShockLoopCuefromAdditionalActor DeadActor)
  (Utilities|Array|RemoveItem (Variables|Default|GetAdditionalTargets) DeadActor))

(fn EnforceImplementsCombatInterface
  (if (Utilities|DoesObjectImplementInterface (Ability|GetAvatarActorfromActorInfo) "/Script/Aura.CombatInterface")
    (return)
    (else
      (Ability|CancelAbility))))

(fn PreparetoEndAbility
  (Variables|/Script/Engine.PlayerController|SetbShowMouseCursor (Variables|Default|GetOwnerPlayerController) true)
  (Class|CombatInterface|SetinShockLoop(Message) (Ability|GetAvatarActorfromActorInfo) false)
  (Pawn|Components|CharacterMovement|SetMovementMode (Variables|/Script/Engine.Character|GetCharacterMovement (Variables|Default|GetOwnerCharacter)) "MOVE_Walking" 0)
  (CallFunction|RemoveAllGameplayCues))

(fn InShockLoop
  (Class|CombatInterface|SetinShockLoop(Message) (Ability|GetAvatarActorfromActorInfo) true)
  (Pawn|Components|CharacterMovement|DisableMovement (Variables|/Script/Engine.Character|GetCharacterMovement (Variables|Default|GetOwnerCharacter))))

(fn PreparetoStartAbility
  (Variables|/Script/Engine.PlayerController|SetbShowMouseCursor (Variables|Default|GetOwnerPlayerController) false)
  (Class|CombatInterface|UpdateFacingTarget(Message) (Ability|GetAvatarActorfromActorInfo) (Variables|Default|GetMouseHitLocation)))

(fn SpawnElectricBeam
  (Class|AuraBeamSpell|TraceFirstTarget (Variables|Default|GetMouseHitLocation) false)
  (bind _returnvalue (Class|CombatInterface|GetWeapon(Message) (Variables|Default|GetOwnerCharacter)))
  (Variables|Default|SetFirstTargetCueParams (Ability|GameplayCue|MakeGameplayCueParameters :Location (Variables|Default|GetMouseHitLocation) :SourceObject (Variables|Default|GetMouseHitActor) :TargetAttachComponent _returnvalue))
  ;[0 1 1] Are we hitting an enemy ?
  (bind _output_get (Variables|Default|SetFirstTargetImplInterface (Utilities|DoesObjectImplementInterface (Variables|Default|GetMouseHitActor) "/Script/Aura.CombatInterface")))
  (if _output_get
    ;[0.7578 0 1] Add the cue to the correct target
    (GameplayCue|AddGameplayCueOnActor(Looping) (Variables|Default|GetMouseHitActor) "(TagName=\"GameplayCue.ShockLoop\")" (Variables|Default|GetFirstTargetCueParams))
    (Class|CombatInterface|SetIsBeingShocked(Message) (Variables|Default|GetMouseHitActor) true)
    ;[0.9922 1 0] Find nearby additional targets, and "grant" them GC_ShockLoop
    (bind _outadditionaltargets (Class|AuraBeamSpell|StoreAdditionalTargets))
    (bind _output_get_2 (Variables|Default|SetAdditionalTargets _outadditionaltargets))
    (for _array_element _output_get_2
      (Class|CombatInterface|SetIsBeingShocked(Message) _array_element true)
      (CallFunction|AddSockLoopCuetoAdditionalActor _array_element))
    (else
      (GameplayCue|AddGameplayCueOnActor(Looping) (Ability|GetAvatarActorfromActorInfo) "(TagName=\"GameplayCue.ShockLoop\")" (Variables|Default|GetFirstTargetCueParams)))))

(fn AddSockLoopCuetoAdditionalActor
  (params (AdditionalActor :type Actor%20Object%20Reference))
  (bind _mousehitactor (Variables|Default|GetMouseHitActor))
  (bind _returnvalue (Transformation|GetActorLocation AdditionalActor))
  (bind _rootcomponent (Variables|/Script/Engine.Actor|GetRootComponent _mousehitactor))
  (bind _returnvalue_2 (Ability|GameplayCue|MakeGameplayCueParameters :Location _returnvalue :SourceObject AdditionalActor :TargetAttachComponent _rootcomponent))
  (Utilities|Map|Add (Variables|Default|GetAdditionalActorsToCueParams) AdditionalActor _returnvalue_2)
  (GameplayCue|AddGameplayCueOnActor(Looping) AdditionalActor "(TagName=\"GameplayCue.ShockLoop\")" _returnvalue_2))

(fn RemoveShockLoopCuefromAdditionalActor
  (params (AdditionalActor :type Actor%20Object%20Reference))
  (bind _additionalactorstocueparams (Variables|Default|GetAdditionalActorsToCueParams))
  (bind (_value _returnvalue) (Utilities|Map|Find _additionalactorstocueparams AdditionalActor))
  (if _returnvalue
    (GameplayCue|RemoveGameplayCueOnActor(Looping) AdditionalActor "(TagName=\"GameplayCue.ShockLoop\")" _value)))

(fn ApplyDamage
  (CallFunction|ApplyDamageSingleTarget (Variables|Default|GetMouseHitActor))
  (for _array_element (Variables|Default|GetAdditionalTargets)
    (CallFunction|ApplyDamageSingleTarget _array_element)))

(fn ApplyDamageSingleTarget
  (params (Actor :type Actor%20Object%20Reference))
  (bind _returnvalue (Ability|GetAbilitySystemComponent Actor))
  (Utilities|IsValid Actor
    (:Is%20Valid
      (if (Class|AuraAbilitySystemLibrary|IsNotFriend Actor (Variables|Default|GetOwnerCharacter))
        (bind _output_get (LocalVariables|SetASC (Ability|GetAbilitySystemComponentfromActorInfo)))
        (Utilities|IsValid _output_get
          (:Is%20Valid
            (bind _returnvalue_2 (Ability|GameplayEffect|AssignTagSetbyCallerMagnitude (GameplayEffects|MakeOutgoingSpec (LocalVariables|GetASC) (Variables|Default|GetDamageEffectClass) (Math|Conversions|ToFloat(Integer) (Ability|GetAbilityLevel)) (GameplayEffects|MakeEffectContext (LocalVariables|GetASC))) "(TagName=\"Damage.Lightning\")" (Class|AuraDamageGameplayAbility|GetDamage (Math|Conversions|ToFloat(Integer) (Ability|GetAbilityLevel)))))
            (Utilities|IsValid _returnvalue
              (:Is%20Valid
                (GameplayEffects|ApplyGameplayEffectSpecToSelf _returnvalue _returnvalue_2)))))))))

(fn ResetKeyVariables
  (Utilities|Array|Clear (Variables|Default|GetAdditionalTargets))
  (Utilities|Map|Clear (Variables|Default|GetAdditionalActorsToCueParams))
  (Variables|Default|SetMouseHitActor 0)
  (Variables|Default|SetFirstTargetImplInterface false)
  (Variables|Default|SetTimeHeld 0.0))

(fn RemoveAllGameplayCues
  ;[0.6875 0 1] Remove the cue depending on if we hit an enemy OR anything else
  (if (Variables|Default|GetFirstTargetImplInterface)
    (GameplayCue|RemoveGameplayCueOnActor(Looping) (Variables|Default|GetMouseHitActor) "(TagName=\"GameplayCue.ShockLoop\")" (Variables|Default|GetFirstTargetCueParams))
    (Class|CombatInterface|SetIsBeingShocked(Message) (Variables|Default|GetMouseHitActor) false)
    (Ability|HasAuthority
      (:True
        ;[0 0.1328 1] Apply damage one last time, but this time including debuff chance
        (CallFunction|ApplyLastDamage (Variables|Default|GetMouseHitActor)))
      (:False
        _))
    ;[1 0 0.6328] Remove GC_ShockLoop from additional targets, if we've hit an enemy
    (for _array_element (Variables|Default|GetAdditionalTargets)
      (Class|CombatInterface|SetIsBeingShocked(Message) _array_element false)
      (CallFunction|RemoveShockLoopCuefromAdditionalActor _array_element)
      (Ability|HasAuthority
        (:True
          ;[0 1 0.3203] Apply damage one last time, but this time including debuff chance
          (CallFunction|ApplyLastDamage _array_element))))
    (return)
    (else
      (GameplayCue|RemoveGameplayCueOnActor(Looping) (Ability|GetAvatarActorfromActorInfo) "(TagName=\"GameplayCue.ShockLoop\")" (Variables|Default|GetFirstTargetCueParams))
      (return))))

(fn GetDescription
  (params (Level :type Integer))
  (return (Utilities|String|ToString(Text) (Utilities|Text|FormatText "<Title>ELECTROCUTE</> 
<Small>Level   </><Level>{Level}</> 
<Small>Mana Cost   </><ManaCost>{ManaCost}</> 
<Small>Cooldown   </><Cooldown>{Cooldown}s</> 
 
<Default>Emits a beam of lightning, {NumAdditionalBeams}, repeatedly causing </><Damage>{Damage}</><Default> lightning damage with a chance to stun.</>" Level (Class|AuraGameplayAbility|GetManaCost (Math|Conversions|ToFloat(Integer) Level)) (Class|AuraGameplayAbility|GetCooldown (Math|Conversions|ToFloat(Integer) Level)) (select (== Level 1) "connecting with the target" (Utilities|String|Append "propagating to </><Number>" (Utilities|String|ToString(Integer) (Math|Integer|Min(Integer) (- Level 1) (Variables|Default|GetMaxNumberOfShockTargets))) "</><Default> additional targets nearby")) (Math|Float|Truncate (Class|AuraDamageGameplayAbility|GetDamage (Math|Conversions|ToFloat(Integer) Level)))))))

(fn GetNextLevelDescription
  (params (Level :type Integer))
  (return (Utilities|String|ToString(Text) (Utilities|Text|FormatText "<Title>ELECTROCUTE</> 
<Small>Level   </><Level>{Level}</> 
<Small>Mana Cost   </><ManaCost>{ManaCost}</> 
<Small>Cooldown   </><Cooldown>{Cooldown}s</> 
 
<Default>Emits a beam of lightning, propagating to </><Number>{NumAdditionalBeams}</><Default> additional targets nearby, repeatedly causing </><Damage>{Damage}</><Default> lightning damage with a chance to stun.</>" Level (Class|AuraGameplayAbility|GetManaCost (Math|Conversions|ToFloat(Integer) Level)) (Class|AuraGameplayAbility|GetCooldown (Math|Conversions|ToFloat(Integer) Level)) (Math|Integer|Min(Integer) (- Level 1) (Variables|Default|GetMaxNumberOfShockTargets)) (Math|Float|Truncate (Class|AuraDamageGameplayAbility|GetDamage (Math|Conversions|ToFloat(Integer) Level)))))))

(fn ClearandEndAbility
  (Utilities|Time|ClearandInvalidateTimerbyHandle (Variables|Default|GetDamageAndCostTimer))
  (CallFunction|PreparetoEndAbility)
  (Ability|CommitAbilityCooldown false)
  (CallFunction|ResetKeyVariables)
  (Ability|EndAbility))

(fn ApplyLastDamage
  (params (TargetActor :type Actor%20Object%20Reference))
  (if (Class|AuraAbilitySystemLibrary|IsNotFriend (Variables|Default|GetOwnerCharacter) TargetActor)
    (Class|AuraAbilitySystemLibrary|ApplyDamageEffect (Class|AuraDamageGameplayAbility|MakeDamageEffectParamsfromClassDefaults TargetActor))))