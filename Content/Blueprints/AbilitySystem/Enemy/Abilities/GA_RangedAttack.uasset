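; GA_RangedAttack is an enemy gameplay ability that fires a projectile at the avatar's combat target.
; It faces the target, plays a random attack montage and waits for that montage's tagged gameplay event.
; On the event it spawns a projectile from the tagged socket toward the target location captured at activation, with optional pitch override from a calculated angle plus offset.
; The ability ends after spawning or when the montage completes, is interrupted or cancelled.
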(event Ability|EventActivateAbility
  (bind _returnvalue (Ability|GetAvatarActorfromActorInfo))
  ;[0.125 1 0] Make the actor face the target
  ;;[1 0 0.8437] Should be set by Behavior tree (BTT_Attack)
  (bind _returnvalue_2 (Class|EnemyInterface|GetCombatTarget(Message) _returnvalue))
  (Variables|Default|SetTargetLocation (Transformation|GetActorLocation _returnvalue_2))
  (Class|CombatInterface|UpdateFacingTarget(Message) _returnvalue (Transformation|GetActorLocation _returnvalue_2))
  ;[0 0.8594 1] Play a random attack animation
  (bind _returnvalue_3 (Class|CombatInterface|GetAttackMontages(Message) _returnvalue))
  (bind _output_get (Variables|Default|SetTaggedMontage (.OutItem (Utilities|Array|Random _returnvalue_3))))
  (|PlayMontageandWaitProxy "None" (.Montage (Utilities|Struct|BreakTaggedMontage _output_get)) 1.0 "None" false 1.0 0.0 false
    (:then
      ;[1 0.8438 0] Wait for the anim notify event
      (Ability|Tasks|WaitGameplayEvent (.MontageTag (Utilities|Struct|BreakTaggedMontage _output_get)) 0 true
        (:EventReceived
          ;[1 0.7734 0] Calculate correction angle
          (bind _returnvalue_4 (Class|CombatInterface|GetCombatSocketLocation(Message) (Ability|GetAvatarActorfromActorInfo) (.SocketTag (Utilities|Struct|BreakTaggedMontage _output_get))))
          ;[0.6875 0 1] Spawn Projectile and End Ability
          (Class|AuraProjectileSpell|SpawnProjectile (Variables|Default|GetTargetLocation) (.SocketTag (Utilities|Struct|BreakTaggedMontage _output_get)) (Variables|Default|GetShouldOverridePitch) (+ (Class|AuraProjectileSpell|CalculatePitch 1e+03 _returnvalue_4 (Variables|Default|GetTargetLocation) 9.81) (Variables|Default|GetAdditivePitch)))
          (Ability|EndAbility))))
    (:OnCompleted
      (Ability|EndAbility :!label _label))
    (:OnInterrupted
      (goto _label))
    (:OnCancelled
      (goto _label))))

(event Ability|EventOnEndAbility
  (params (bWasCancelled :type Boolean)))